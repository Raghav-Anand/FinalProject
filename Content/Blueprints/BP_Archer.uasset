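; BP_Archer is a 2D flipbook archer character that shoots arrows and dies from one hit by an attacking BP_SpriteCharacter.
; Tick snaps rotation to two facings by yaw, picks the Death, Shoot, run or Idle flipbook, and polls HitBox overlaps for attackers.
; Overlap begin also applies damage; health loss triggers a delayed destroy.
; Fire, not called within this graph, spawns BP_Arrow after a shooting delay.
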(event `self.ReceiveBeginPlay`)

(event `Get Rotation`)

(event `self.ReceiveTick`
  (params (DeltaSeconds :type "Float (single-precision)"))
  (bind (_returnvalue_roll _returnvalue_pitch _returnvalue_yaw) (`KismetMathLibrary.BreakRotator` (`self.K2_GetActorRotation`)))
  (if (<= _returnvalue_yaw 90.0)
    (`self.K2_SetActorRotation` (struct))
    (else
      (`self.K2_SetActorRotation` (struct :`Yaw` 180.0))))
  (`self.UpdateAnimation`)
  (for _array_element (`PrimitiveComponent.GetOverlappingActors` (`self.HitBox`) "/Game/Blueprints/BP_SpriteCharacter.BP_SpriteCharacter_C")
    (bind _asbp_sprite_character (cast `/Game/Blueprints/BP_SpriteCharacter` _array_element))
    (if (`/Game/Blueprints/BP_SpriteCharacter.Is Attacking` _asbp_sprite_character)
      (`self.UpdateHealth` -1.0))))

(event `Fire`
  (set `self.Is Shooting` true)
  (`KismetSystemLibrary.Delay` 0.6)
  (set `self.Is Shooting` false)
  (bind _returnvalue (`|SpawnActorFromClass` "/Game/Blueprints/BP_Arrow.BP_Arrow_C" (`KismetMathLibrary.MakeTransform` (`self.K2_GetActorLocation`)) "Undefined" "MultiplyWithRoot" null null))
  (`KismetSystemLibrary.PrintString` (`KismetSystemLibrary.GetDisplayName` _returnvalue))
  (`KismetSystemLibrary.Delay` 1.0))

(event `UpdateHealth`
  (params (Delta :type "Float (double-precision)"))
  (bind _output_get (set `self.HP` (`KismetMathLibrary.FClamp` (+ Delta (`self.HP`)) 0.0 1.0)))
  (if (<= _output_get 0.0)
    (set `self.Is Dead` true)
    (`KismetSystemLibrary.Delay` 1.0667)
    (`self.K2_DestroyActor`)))

(event `UpdateAnimation`
  (`PaperFlipbookComponent.SetFlipbook` (`self.Sprite`) (select `bool` (`self.Is Dead`) :`false` (select `bool` (`self.Is Shooting`) :`false` (select `bool` (> (`KismetMathLibrary.VSize` (`MovementComponent.Velocity` (`self.CharacterMovement`))) 0.0) :`false` "/Game/ArcherEnemy/Idle/Idle.Idle" :`true` "/Game/ArcherEnemy/Run/ArcherRun.ArcherRun" :!type "PaperFlipbook Object Reference") :`true` "/Game/ArcherEnemy/Shoot/Shoot.Shoot") :`true` "/Game/ArcherEnemy/Death/Death.Death")))

(event `self.HitBox.OnComponentBeginOverlap`
  (params (OverlappedComponent :type "PrimitiveComponent Object Reference") (OtherActor :type "Actor Object Reference") (OtherComp :type "PrimitiveComponent Object Reference") (OtherBodyIndex :type Integer) (bFromSweep :type Boolean) (SweepResult :type "HitResult Structure (by ref)"))
  (bind _asbp_sprite_character (cast `/Game/Blueprints/BP_SpriteCharacter` OtherActor))
  (`KismetSystemLibrary.PrintString` "Hello")
  (if (`/Game/Blueprints/BP_SpriteCharacter.Is Attacking` _asbp_sprite_character)
    (`self.UpdateHealth` -1.0)))

(fn `UserConstructionScript`)