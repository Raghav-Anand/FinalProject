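; BP_Arrow is an arrow projectile that launches itself at the player on spawn and damages BP_SpriteCharacter on overlap.
; BeginPlay leads the player by distance over speed times player velocity, then sets ProjectileMovement from a suggested ballistic toss velocity, with debug drawing on and rotation following velocity.
; Overlapping a BP_SpriteCharacter reduces its health and destroys the arrow.
; Any other overlap also destroys it, except BP_Archer, which is ignored.
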(event `self.ReceiveBeginPlay`
  (bind _returnvalue (`GameplayStatics.GetPlayerCharacter` 0))
  (bind _projectilemovement (`self.ProjectileMovement`))
  (bind _tossvelocity (`GameplayStatics.BlueprintSuggestProjectileVelocity` (`self.K2_GetActorLocation`) (+ (`self.K2_GetActorLocation` _returnvalue) (* (/ (`self.GetDistanceTo` _returnvalue) (`self.Speed`)) (`self.GetVelocity` _returnvalue))) (`self.Speed`) 0.0 "DoNotTrace" 0.0 false true))
  (set `MovementComponent.Velocity` _tossvelocity _projectilemovement)
  (set `ProjectileMovementComponent.bRotationFollowsVelocity` true _projectilemovement))

(event `self.ReceiveActorBeginOverlap`
  (params (OtherActor :type "Actor Object Reference"))
  (bind _asbp_sprite_character (cast `/Game/Blueprints/BP_SpriteCharacter` OtherActor)
    (:`then`
      (`/Game/Blueprints/BP_SpriteCharacter.UpdateHealth` _asbp_sprite_character -0.5))
    (:`CastFailed`
      (cast `/Game/Blueprints/BP_Archer` OtherActor
        (:`CastFailed`
          _))))
  (`self.K2_DestroyActor`))

(fn `UserConstructionScript`)