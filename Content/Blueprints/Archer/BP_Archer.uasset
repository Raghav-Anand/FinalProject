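; BP_Archer is a Paper2D archer character that shoots arrows, takes health changes and dies.
; Tick snaps its rotation to one of two side-on facings based on yaw, then picks a death, shoot, run or idle flipbook from state and velocity.
; Fire holds the shooting state briefly before spawning BP_Arrow at the archer's location.
; UpdateHealth clamps normalized HP and, at zero, delays destruction for the death animation.
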(event `self.ReceiveBeginPlay`)

(event `Get Rotation`)

(event `self.ReceiveTick`
  (params (DeltaSeconds :type "Float (single-precision)"))
  (bind (_returnvalue_roll _returnvalue_pitch _returnvalue_yaw) (`KismetMathLibrary.BreakRotator` (`self.K2_GetActorRotation`)))
  (if (<= _returnvalue_yaw 90.0)
    (`self.K2_SetActorRotation` (struct))
    (else
      (`self.K2_SetActorRotation` (struct :`Yaw` 180.0))))
  (`self.UpdateAnimation`))

(event `Fire`
  (set `self.Is Shooting` true)
  (`KismetSystemLibrary.Delay` 0.6)
  (set `self.Is Shooting` false)
  (`|SpawnActorFromClass` "/Game/Blueprints/Archer/BP_Arrow.BP_Arrow_C" (`KismetMathLibrary.MakeTransform` (`self.K2_GetActorLocation`)) "Undefined" "MultiplyWithRoot" null null)
  (`KismetSystemLibrary.Delay` 1.0))

(event `UpdateHealth`
  (params (Delta :type "Float (double-precision)"))
  (bind _output_get (set `self.HP` (`KismetMathLibrary.FClamp` (+ Delta (`self.HP`)))))
  (if (<= _output_get 0.0)
    (set `self.Is Dead` true)
    (`KismetSystemLibrary.Delay` 1.0667)
    (`self.K2_DestroyActor`)))

(event `UpdateAnimation`
  (`PaperFlipbookComponent.SetFlipbook` (`self.Sprite`) (select `bool` (`self.Is Dead`) :`false` (select `bool` (`self.Is Shooting`) :`false` (select `bool` (> (`KismetMathLibrary.VSize` (`MovementComponent.Velocity` (`self.CharacterMovement`))) 0.0) :`false` "/Game/ArcherEnemy/Idle/Idle.Idle" :`true` "/Game/ArcherEnemy/Run/ArcherRun.ArcherRun" :!type "PaperFlipbook Object Reference") :`true` "/Game/ArcherEnemy/Shoot/Shoot.Shoot") :`true` "/Game/ArcherEnemy/Death/Death.Death")))

(fn `UserConstructionScript`)